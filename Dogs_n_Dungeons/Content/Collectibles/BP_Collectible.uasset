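; Pickup actor that restores either health or mana to the BP_ZaZaCat player, depending on its CollectibleType.
; The construction script shows the matching mesh, and BeginPlay sets that mesh's collision and bobbing values.
; A looping timer bobs the mesh on a sine wave around the health mesh's starting relative location.
; On overlap it adds the clamped amount, notifies the player, plays a sound and destroys itself, unless that stat is full.
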(event `CollectibleTypeVariables`
  (bind _healthcollectible (`self.HealthCollectible`))
  (bind _manacollectible (`self.ManaCollectible`))
  ;[0 0.1559 0.1274] Based on collectible type, change bobbing speed, distance, what mesh will be bobbing, and mesh collision.
  (switch `/Game/Collectibles/E_CollectibleTypes` (`self.CollectibleType`)
    (:`NewEnumerator0`
      (set `self.BobbingSpeed` (`self.HealthBobbingSpeed`))
      (set `self.BobbingDistance` (`self.HealthBobbingDistance`))
      (set `self.MeshToBob` _healthcollectible)
      (`PrimitiveComponent.SetCollisionEnabled` _healthcollectible "QueryAndPhysics")
      (`PrimitiveComponent.SetCollisionEnabled` (`self.ManaCollectible`) "NoCollision"))
    (:`NewEnumerator1`
      (set `self.BobbingSpeed` (`self.ManaBobbingSpeed`))
      (set `self.BobbingDistance` (`self.ManaBobbingDistance`))
      (set `self.MeshToBob` _manacollectible)
      (`PrimitiveComponent.SetCollisionEnabled` _manacollectible "QueryAndPhysics")
      (`PrimitiveComponent.SetCollisionEnabled` (`self.HealthCollectible`) "NoCollision"))))

(event `self.ReceiveBeginPlay`
  (`self.CollectibleTypeVariables`)
  ;[0.9734 0.5776 0.01681] Sets Timer and Relative Location for Bobbing Effect
  (`KismetSystemLibrary.K2_SetTimer` null "BobbingEffect" 0.01 true)
  (set `self.RelativeLocation` (`SceneComponent.RelativeLocation` (`self.HealthCollectible`))))

(event `BobbingEffect`
  (bind (_relativelocation_x _relativelocation_y _relativelocation_z) (`KismetMathLibrary.BreakVector` (`self.RelativeLocation`)))
  ;[0.956 0.5647 0.01681] Bobbing Effect
  (`SceneComponent.K2_SetRelativeLocation` (`self.MeshToBob`) (`KismetMathLibrary.MakeVector` _relativelocation_x _relativelocation_y (+ _relativelocation_z (* (`KismetMathLibrary.DegSin` (* (`self.GetGameTimeSinceCreation`) (`self.BobbingSpeed`))) (`self.BobbingDistance`)))) false false))

(event `self.HealthCollectible.OnComponentBeginOverlap`
  (params (OverlappedComponent :type "PrimitiveComponent Object Reference") (OtherActor :type "Actor Object Reference") (OtherComp :type "PrimitiveComponent Object Reference") (OtherBodyIndex :type Integer) (bFromSweep :type Boolean) (SweepResult :type "HitResult Structure (by ref)"))
  ;[0.03955 0.6584 0] Changes Player's Health
  (bind _asbp_za_za_cat (cast `/Game/DefaultShit/ThirdPerson/Blueprints/BP_ZaZaCat` OtherActor))
  (bind _maxhealth (`/Game/DefaultShit/ThirdPerson/Blueprints/BP_ZaZaCat.MaxHealth` _asbp_za_za_cat))
  ;;[0.03955 0.6584 0] Make sure player is not at max health. If they are, do nothing (collectible isn't picked up).
  (if (!= (`/Game/DefaultShit/ThirdPerson/Blueprints/BP_ZaZaCat.Health` _asbp_za_za_cat) _maxhealth)
    (bind _output_get (set `/Game/DefaultShit/ThirdPerson/Blueprints/BP_ZaZaCat.Health` (`KismetMathLibrary.FClamp` (+ (`/Game/DefaultShit/ThirdPerson/Blueprints/BP_ZaZaCat.Health` _asbp_za_za_cat) (`self.HealthGained`)) 0.0 _maxhealth) _asbp_za_za_cat))
    (`/Game/DefaultShit/ThirdPerson/Blueprints/BP_ZaZaCat.HealthChanged` _asbp_za_za_cat _output_get)
    (`GameplayStatics.PlaySound2D` "/Engine/EngineSounds/1kSineTonePing.1kSineTonePing" 1.0 1.0 0.0 null null)
    (`self.K2_DestroyActor`)))

(event `self.ManaCollectible.OnComponentBeginOverlap`
  (params (OverlappedComponent :type "PrimitiveComponent Object Reference") (OtherActor :type "Actor Object Reference") (OtherComp :type "PrimitiveComponent Object Reference") (OtherBodyIndex :type Integer) (bFromSweep :type Boolean) (SweepResult :type "HitResult Structure (by ref)"))
  ;[0.03955 0.6584 0] Changes Player's Mana
  (bind _asbp_za_za_cat (cast `/Game/DefaultShit/ThirdPerson/Blueprints/BP_ZaZaCat` OtherActor))
  (bind _maxmana (`/Game/DefaultShit/ThirdPerson/Blueprints/BP_ZaZaCat.MaxMana` _asbp_za_za_cat))
  ;;[0.03955 0.6584 0] Make sure player is not at max mana. If they are, do nothing (collectible isn't picked up).
  (if (!= (`/Game/DefaultShit/ThirdPerson/Blueprints/BP_ZaZaCat.Mana` _asbp_za_za_cat) _maxmana)
    (bind _output_get (set `/Game/DefaultShit/ThirdPerson/Blueprints/BP_ZaZaCat.Mana` (`KismetMathLibrary.FClamp` (+ (`/Game/DefaultShit/ThirdPerson/Blueprints/BP_ZaZaCat.Mana` _asbp_za_za_cat) (`self.ManaGained`)) 0.0 _maxmana) _asbp_za_za_cat))
    (`/Game/DefaultShit/ThirdPerson/Blueprints/BP_ZaZaCat.ManaChanged` _asbp_za_za_cat _output_get)
    (`GameplayStatics.PlaySound2D` "/Engine/EditorSounds/Notifications/CompileFailed.CompileFailed" 1.0 1.0 0.0 null null)
    (`self.K2_DestroyActor`)))

(fn `UserConstructionScript`
  (switch `/Game/Collectibles/E_CollectibleTypes` (`self.CollectibleType`)
    (:`NewEnumerator0`
      (`SceneComponent.SetVisibility` (`self.HealthCollectible`) true false)
      (`SceneComponent.SetVisibility` (`self.ManaCollectible`) false false))
    (:`NewEnumerator1`
      (`SceneComponent.SetVisibility` (`self.ManaCollectible`) true false)
      (`SceneComponent.SetVisibility` (`self.HealthCollectible`) false false))))