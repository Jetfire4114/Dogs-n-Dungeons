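; BP_TeslaCoil is a puzzle coil that becomes active when electrified and passes electricity on to nearby objects.
; Electrified registers the coil in the game mode's activated list, notifies the game mode, enables TransferRadius query collision and starts the Lightning effect.
; Overlaps with TransferRadius send the electrify message to BPI_Electrifiable actors, allowing chain reactions.
; CoilUnactivated only stops the Lightning effect, leaving collision and registration untouched.
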(event `self.ReceiveBeginPlay`
  (bind _asbp_third_person_game_mode (cast `/Game/DefaultShit/ThirdPerson/Blueprints/BP_ThirdPersonGameMode` (`GameplayStatics.GetGameMode`)))
  (set `self.GameModeRef` _asbp_third_person_game_mode))

(event `/Game/PuzzleThings/BPI_Electrifiable.Electrified`
  (`self.CoilActivated`)
  (`PrimitiveComponent.SetCollisionEnabled` (`self.TransferRadius`) "QueryOnly")
  (`ActorComponent.Activate` (`self.Lightning`) false))

(event `/Game/PuzzleThings/BPI_Electrifiable.CoilActivated`
  (bind _gamemoderef (`self.GameModeRef`))
  (`KismetArrayLibrary.Array_AddUnique` (`/Game/DefaultShit/ThirdPerson/Blueprints/BP_ThirdPersonGameMode.ActivatedTeslaCoils` _gamemoderef) self)
  (`/Game/DefaultShit/ThirdPerson/Blueprints/BP_ThirdPersonGameMode.CoilActivated` _gamemoderef))

(event `/Game/PuzzleThings/BPI_Electrifiable.CoilUnactivated`
  (`ActorComponent.Deactivate` (`self.Lightning`)))

(event `self.TransferRadius.OnComponentBeginOverlap`
  (params (OverlappedComponent :type "PrimitiveComponent Object Reference") (OtherActor :type "Actor Object Reference") (OtherComp :type "PrimitiveComponent Object Reference") (OtherBodyIndex :type Integer) (bFromSweep :type Boolean) (SweepResult :type "HitResult Structure (by ref)"))
  (if (`KismetSystemLibrary.DoesImplementInterface` OtherActor "/Game/PuzzleThings/BPI_Electrifiable.BPI_Electrifiable_C")
    (message `/Game/PuzzleThings/BPI_Electrifiable.Electrified` OtherActor)))

(fn `UserConstructionScript`)