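; BP_Torch is a puzzle torch that registers as lit when burned and can pass fire to burnable actors.
; Burned fires TorchLit, which adds the torch to BP_ThirdPersonGameMode's ActivatedTorches and notifies the game mode, then enables query collision on TransferRadius.
; Overlapping actors implementing BPI_Burnable receive BurnedMessage, allowing fire to spread.
; TorchUnlit only prints debug text; the node removing the torch from the list is unconnected.
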(event `self.ReceiveBeginPlay`
  (bind _asbp_third_person_game_mode (cast `/Game/DefaultShit/ThirdPerson/Blueprints/BP_ThirdPersonGameMode` (`GameplayStatics.GetGameMode`)))
  (set `self.GameModeRef` _asbp_third_person_game_mode))

(event `/Game/PuzzleThings/BPI_Burnable.Burned`
  (`self.TorchLit`)
  (`PrimitiveComponent.SetCollisionEnabled` (`self.TransferRadius`) "QueryOnly"))

(event `/Game/PuzzleThings/BPI_Burnable.TorchLit`
  (bind _gamemoderef (`self.GameModeRef`))
  (bind _returnvalue (`KismetArrayLibrary.Array_AddUnique` (`/Game/DefaultShit/ThirdPerson/Blueprints/BP_ThirdPersonGameMode.ActivatedTorches` _gamemoderef) self))
  (`/Game/DefaultShit/ThirdPerson/Blueprints/BP_ThirdPersonGameMode.TorchLit` _gamemoderef)
  (`KismetSystemLibrary.PrintString` (`KismetStringLibrary.Concat_StrStr` "torch lit, index: " (`KismetStringLibrary.Conv_IntToString` _returnvalue))))

(event `/Game/PuzzleThings/BPI_Burnable.TorchUnlit`
  (`KismetSystemLibrary.PrintString` "unlit"))

(event `self.TransferRadius.OnComponentBeginOverlap`
  (params (OverlappedComponent :type "PrimitiveComponent Object Reference") (OtherActor :type "Actor Object Reference") (OtherComp :type "PrimitiveComponent Object Reference") (OtherBodyIndex :type Integer) (bFromSweep :type Boolean) (SweepResult :type "HitResult Structure (by ref)"))
  (if (`KismetSystemLibrary.DoesImplementInterface` OtherActor "/Game/PuzzleThings/BPI_Burnable.BPI_Burnable_C")
    (message `/Game/PuzzleThings/BPI_Burnable.Burned` OtherActor)))

(fn `UserConstructionScript`)