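; BP_EnemyDog is an enemy that chases seen pawns and attacks on arrival, currently with placeholder animation and zero damage, then stuns itself.
; PawnSensing starts a repeating follow timer using AI MoveTo; each sighting restarts a timeline that drops the target and stops the dog when it finishes.
; A matching-element hit stuns it, temporarily swapping its material; health changes apply only while stunned.
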(event `self.PawnSensing.OnSeePawn`
  (params (Pawn :type "Pawn Object Reference"))
  (`|ExecutionSequence`
    (:`then_0`
      ;[1 1 1] If Player Not Seen within Timeline Length, stop Enemy
      (`Timeline|PlayerNotSeen` :!via `PlayFromStart`
        (:`Finished`
          (set `self.Player` null)
          (`KismetSystemLibrary.K2_ClearAndInvalidateTimerHandle` (`self.FollowPlayerTimer`))
          (`MovementComponent.StopMovementImmediately` (`self.CharacterMovement`)))))
    (:`then_1`
      (set `self.Player` Pawn)
      (bind _returnvalue (`KismetSystemLibrary.K2_SetTimer` null "FollowPlayer" 0.2 true))
      (set `self.FollowPlayerTimer` _returnvalue))))

(event `FollowPlayer`
  (if (`KismetSystemLibrary.IsValid` (`self.Player`))
    (if (not (`self.IsStunned`))
      (set `self.CanAttack` true)
      (`|AIMoveTo` self (0.0 0.0 0.0) (`self.Player`) 70.0
        (:`OnSuccess`
          (if (`self.CanAttack`)
            (set `self.CanAttack` false)
            ;[1 1 1] Future Attack Animation
            (`self.PlayAnimMontage` null)
            (`KismetSystemLibrary.Delay` 0.2)
            (set `self.CanAttack` true)
            (message `/Game/Users/Michael/Enemies/BPI_Health.ChangeHealth` (`self.Player`) 0.0 "NewEnumerator0")
            (`KismetSystemLibrary.PrintString` "attacking")
            (`self.StunEnemy`)))))))

(event `/Game/Users/Michael/Enemies/BPI_Health.ChangeHealth`
  (params (HealthChange :type "Float (double-precision)") (Element :type "/Game/Users/Michael/Enemies/E_Element Enum" :default "NewEnumerator0"))
  (if (`self.IsStunned`)
    (set `self.Health` (+ (`self.Health`) HealthChange))
    (elif (`|EnumEquality` Element (`self.ElementState`))
      (`self.StunEnemy`))))

(event `StunEnemy`
  (set `self.IsStunned` true)
  (`PrimitiveComponent.SetMaterial` (`self.Mesh`) 0 "/Engine/VREditor/UI/DiscMaterial.DiscMaterial")
  (`NavMovementComponent.StopActiveMovement` (`self.CharacterMovement`))
  (`KismetSystemLibrary.Delay` (`self.StunDuration`))
  (set `self.IsStunned` false)
  (`PrimitiveComponent.SetMaterial` (`self.Mesh`) 0 "/Game/Users/Luke/Colors/EnemyDog.EnemyDog"))

(fn `UserConstructionScript`)