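; BP_HatPlatform is a moving platform that makes one round trip when a ChangeHealth event delivers a specific element while it is idle.
; A Movement timeline lerps the platform's height from start to end marker, pauses, then reverses.
; The timeline also offsets CollisionCone downward, using a separate track going forward and the platform's track returning.
; PlatformArms collision is disabled during the return and restored afterward.
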(event `self.ReceiveBeginPlay`
  (set `self.ConeInitialLocation` (`SceneComponent.RelativeLocation` (`self.CollisionCone`)))
  (`SceneComponent.K2_SetWorldLocation` (`self.Platform`) (`SceneComponent.K2_GetComponentLocation` (`self.StartPosition`)) false false))

(event `/Game/Users/Michael/Enemies/BPI_Health.ChangeHealth`
  (params (HealthChange :type "Float (double-precision)") (Element :type "/Game/Users/Michael/Enemies/E_Element Enum" :default "NewEnumerator0"))
  (if (`self.IsActive`)
    _
    (elif (`|EnumEquality` Element "NewEnumerator2")
      (set `self.IsActive` true)
      (`self.ForwardPlatform`))))

(event `ForwardPlatform`
  (bind (_coneinitiallocation_x _coneinitiallocation_y _coneinitiallocation_z) (`KismetMathLibrary.BreakVector` (`self.ConeInitialLocation`)))
  (bind (_returnvalue_x _returnvalue_y _returnvalue_z) (`KismetMathLibrary.BreakVector` (`SceneComponent.K2_GetComponentLocation` (`self.EndPosition`))))
  (bind (_returnvalue_x_2 _returnvalue_y_2 _returnvalue_z_2) (`KismetMathLibrary.BreakVector` (`SceneComponent.K2_GetComponentLocation` (`self.StartPosition`))))
  (bind (_returnvalue_x_3 _returnvalue_y_3) (`KismetMathLibrary.BreakVector` (`SceneComponent.K2_GetComponentLocation` (`self.Platform`))))
  (bind (_relativelocation_x _relativelocation_y) (`KismetMathLibrary.BreakVector` (`SceneComponent.RelativeLocation` (`self.CollisionCone`))))
  ;[1 1 1] Moves Platform and Collision Cone Up and Down
  (bind (_direction _platform _coneforward) (`Timeline|Movement` :!via `PlayFromStart` :!label _label)
    (:`Update`
      (`SceneComponent.K2_SetWorldLocation` (`self.Platform`) (`KismetMathLibrary.MakeVector` _returnvalue_x_3 _returnvalue_y_3 (`KismetMathLibrary.Lerp` _returnvalue_z_2 _returnvalue_z _platform)) false false)
      (`SceneComponent.K2_SetRelativeLocation` (`self.CollisionCone`) (`KismetMathLibrary.MakeVector` _relativelocation_x _relativelocation_y (`KismetMathLibrary.Lerp` _coneinitiallocation_z (- _coneinitiallocation_z 720.0) (select `bool` (`|EnumEquality` _direction "Forward") :`false` _platform :`true` _coneforward))) false false))
    (:`Finished`
      (if (`|EnumEquality` _direction "Forward")
        (`KismetSystemLibrary.Delay` 3.0)
        (`self.ReversePlatform`)
        (else
          (set `self.IsActive` false)
          (`PrimitiveComponent.SetCollisionEnabled` (`self.PlatformArms`) "QueryAndPhysics"))))))

(event `ReversePlatform`
  ;[1 1 1] Moves Platform and Collision Cone Up and Down
  (`PrimitiveComponent.SetCollisionEnabled` (`self.PlatformArms`) "NoCollision")
  (goto _label :!via `ReverseFromEnd`))

(fn `UserConstructionScript`)